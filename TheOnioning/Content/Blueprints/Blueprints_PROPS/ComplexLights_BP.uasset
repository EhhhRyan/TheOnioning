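; ComplexLights_BP is a wall light prop that switches between lit and unlit states based on the LightOn boolean.
; Every Tick it calls LightOn or LightOff, which set the visibility of BottomLight and TopLight and swap the mesh's second material slot between glow and no-glow materials.
; The state is reapplied each frame rather than on change, and the graph's own note flags this as causing frame-time spikes.
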(event Custom|LightOff
  ;[1 0 0.006975] Light On/Off Toggle (NEEDS TO BE MORE OPTIMIZED CAUSES SPIKES IN MS, AND FRAMERATE)
  (Rendering|SetVisibility (Variables|Default|GetBottomLight) false false)
  (Rendering|Material|SetMaterial (Variables|Default|GetStaticMesh) 1 "/Game/Models/ApartmentWallLights/ComplexWallLightNOGLOW_MAT.ComplexWallLightNOGLOW_MAT"))

(event Custom|LightOn
  ;[1 0 0.006975] Light On/Off Toggle (NEEDS TO BE MORE OPTIMIZED CAUSES SPIKES IN MS, AND FRAMERATE)
  (Rendering|SetVisibility (Variables|Default|GetBottomLight) true false)
  (Rendering|Material|SetMaterial (Variables|Default|GetStaticMesh) 1 "/Game/Models/ApartmentWallLights/ComplexWallLightGLOW_MAT.ComplexWallLightGLOW_MAT"))

(event EventTick
  (params (DeltaSeconds :type Float%20%28single-precision%29))
  ;[1 0 0.006975] Light On/Off Toggle (NEEDS TO BE MORE OPTIMIZED CAUSES SPIKES IN MS, AND FRAMERATE)
  (if (Variables|Default|GetLightOn?)
    (CallFunction|Lighton)
    (else
      (CallFunction|LightOff))))

(fn ConstructionScript)